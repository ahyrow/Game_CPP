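; BP_Player is the player actor, which drops a BP_SpawnPoint at its own location when play begins.
; Tick and the construction script are empty.
; A disconnected node chain would rotate the actor toward the point under the mouse cursor, using a visibility trace from BP_PC with Z flattened to zero, but it never runs.
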(event EventBeginPlay
  (Game|SpawnActorfromClass "/Game/BP_SpawnPoint.BP_SpawnPoint_C" (Math|Transform|MakeTransform (Transformation|GetActorLocation) "0, 0, 0" "1.000000,1.000000,1.000000") "Undefined" 0 0))

(event EventTick
  (params (DeltaSeconds :type Float%20%28single-precision%29)))

(fn ConstructionScript)